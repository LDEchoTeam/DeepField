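; Resource container that holds amounts of five ores and five resources, with size, empty check, blended color and display text.
; FillUp adds one ore type through tier-curve weighted random branches, setting its amount from richness and size curves.
; Take and Put move amounts at per-type rates scaled by delta time, and Take returns the remaining amounts.
; GetColor blends type colors by share, while Format builds rounded text but leaves Cibron blank.
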(fn `FillUp`
  (params (Tier :type "Float (double-precision)"))
  (bind _richness (`self.Richness`))
  (bind _returnvalue (`CurveFloat.GetFloatValue` (`self.Ore0Distribution`) Tier))
  (bind _returnvalue_2 (`CurveFloat.GetFloatValue` (`self.SizeDistribution`) (`KismetMathLibrary.RandomFloatInRange` 0.0 1.0)))
  (bind _returnvalue_3 (`CurveFloat.GetFloatValue` (`self.Ore1Distribution`) Tier))
  (bind _returnvalue_4 (`CurveFloat.GetFloatValue` (`self.Ore2Distribution`) Tier))
  (bind _returnvalue_5 (`CurveFloat.GetFloatValue` (`self.Ore3Distribution`) Tier))
  (bind _returnvalue_6 (+ _returnvalue _returnvalue_3))
  (bind _returnvalue_7 (`KismetMathLibrary.RandomFloatInRange` 0.0 (+ _returnvalue _returnvalue_3 _returnvalue_4 _returnvalue_5 (`CurveFloat.GetFloatValue` (`self.Ore4Distribution`) Tier))))
  (bind _returnvalue_8 (+ _returnvalue_6 _returnvalue_4))
  (if (< _returnvalue_7 _returnvalue)
    (set `self.Regolith` (* _richness (`CurveFloat.GetFloatValue` (`self.Ore0SizeDistribution`) Tier) _returnvalue_2))
    (elif (< _returnvalue_7 _returnvalue_6)
      (set `self.Irbonite` (* _richness (`CurveFloat.GetFloatValue` (`self.Ore1SizeDistribution`) Tier) _returnvalue_2))
      (elif (< _returnvalue_7 _returnvalue_8)
        (set `self.Magnesite` (* _richness (`CurveFloat.GetFloatValue` (`self.Ore2SizeDistribution`) Tier) _returnvalue_2))
        (elif (< _returnvalue_7 (+ _returnvalue_8 _returnvalue_5))
          (set `self.Titalumite` (* _richness (`CurveFloat.GetFloatValue` (`self.Ore3SizeDistribution`) Tier) _returnvalue_2))
          (else
            (set `self.Auplatite` (* _richness (`CurveFloat.GetFloatValue` (`self.Ore4SizeDistribution`) Tier) _returnvalue_2)))))))
  (return))

(fn `Format`
  (set `self.FormattedOre0` (`KismetTextLibrary.Conv_DoubleToText` (`self.Regolith`) "HalfToEven" false false 1 2 1 1))
  (set `self.FormattedOre1` (`KismetTextLibrary.Conv_DoubleToText` (`self.Irbonite`) "HalfToEven" false false 1 2 1 1))
  (set `self.FormattedOre2` (`KismetTextLibrary.Conv_DoubleToText` (`self.Magnesite`) "HalfToEven" false false 1 2 1 1))
  (set `self.FormattedOre3` (`KismetTextLibrary.Conv_DoubleToText` (`self.Titalumite`) "HalfToEven" false false 1 2 1 1))
  (set `self.FormattedOre4` (`KismetTextLibrary.Conv_DoubleToText` (`self.Auplatite`) "HalfToEven" false false 1 2 1 1))
  (set `self.FormattedResource0` (`KismetTextLibrary.Conv_DoubleToText` (`self.Filler`) "HalfToEven" false false 1 2 1 1))
  (set `self.FormattedResource1` "")
  (set `self.FormattedResource2` (`KismetTextLibrary.Conv_DoubleToText` (`self.Magnum`) "HalfToEven" false false 1 2 1 1))
  (set `self.FormattedResource3` (`KismetTextLibrary.Conv_DoubleToText` (`self.Alutanium`) "HalfToEven" false false 1 2 1 1))
  (set `self.FormattedResource4` (`KismetTextLibrary.Conv_DoubleToText` (`self.Platigol`) "HalfToEven" false false 1 2 1 1))
  (return))

(fn `GetColor`
  (returns (Color :type "Color Structure"))
  (bind _returnvalue (+ (`self.Regolith`) (`self.Irbonite`) (`self.Magnesite`) (`self.Titalumite`) (`self.Auplatite`) (`self.Filler`) (`self.Cibron`) (`self.Magnum`) (`self.Alutanium`) (`self.Platigol`)))
  (return (`KismetMathLibrary.Conv_LinearColorToColor` (+ (+ (+ (+ (+ (+ (+ (+ (+ (* (`KismetMathLibrary.Conv_ColorToLinearColor` (`self.Ore0Color`)) (/ (`self.Regolith`) _returnvalue)) (* (`KismetMathLibrary.Conv_ColorToLinearColor` (`self.Ore1Color`)) (/ (`self.Irbonite`) _returnvalue))) (* (`KismetMathLibrary.Conv_ColorToLinearColor` (`self.Ore2Color`)) (/ (`self.Magnesite`) _returnvalue))) (* (`KismetMathLibrary.Conv_ColorToLinearColor` (`self.Ore3Color`)) (/ (`self.Titalumite`) _returnvalue))) (* (`KismetMathLibrary.Conv_ColorToLinearColor` (`self.Ore4Color`)) (/ (`self.Auplatite`) _returnvalue))) (* (`KismetMathLibrary.Conv_ColorToLinearColor` (`self.Resource0Color`)) (/ (`self.Filler`) _returnvalue))) (* (`KismetMathLibrary.Conv_ColorToLinearColor` (`self.Resource1Color`)) (/ (`self.Cibron`) _returnvalue))) (* (`KismetMathLibrary.Conv_ColorToLinearColor` (`self.Resource2Color`)) (/ (`self.Magnum`) _returnvalue))) (* (`KismetMathLibrary.Conv_ColorToLinearColor` (`self.Resource3Color`)) (/ (`self.Alutanium`) _returnvalue))) (* (`KismetMathLibrary.Conv_ColorToLinearColor` (`self.Resource4Color`)) (/ (`self.Platigol`) _returnvalue))))))

(fn `GetSize`
  (returns (Size :type "Float (double-precision)"))
  (return (+ (`self.Regolith`) (`self.Irbonite`) (`self.Magnesite`) (`self.Titalumite`) (`self.Auplatite`) (`self.Filler`) (`self.Cibron`) (`self.Magnum`) (`self.Alutanium`) (`self.Platigol`))))

(fn `IsEmpty`
  (returns (Yes :type Boolean))
  (bind _size (`self.GetSize`))
  (return (< _size 0.0001)))

(fn `Put`
  (params (Ore0 :type "Float (double-precision)") (Ore1 :type "Float (double-precision)") (Ore2 :type "Float (double-precision)") (Ore3 :type "Float (double-precision)") (Ore4 :type "Float (double-precision)") (Resource0 :type "Float (double-precision)") (Resource1 :type "Float (double-precision)") (Resource2 :type "Float (double-precision)") (Resource3 :type "Float (double-precision)") (Resource4 :type "Float (double-precision)"))
  (bind _returnvalue (`GameplayStatics.GetWorldDeltaSeconds`))
  (set `self.Regolith` (+ (`self.Regolith`) (`KismetMathLibrary.FClamp` (* (`self.Rate`) (`self.Ore0Rate`) _returnvalue) 0.0 Ore0)))
  (set `self.Irbonite` (+ (`self.Irbonite`) (`KismetMathLibrary.FClamp` (* (`self.Rate`) (`self.Ore1Rate`) _returnvalue) 0.0 Ore1)))
  (set `self.Magnesite` (+ (`self.Magnesite`) (`KismetMathLibrary.FClamp` (* (`self.Rate`) (`self.Ore2Rate`) _returnvalue) 0.0 Ore2)))
  (set `self.Titalumite` (+ (`self.Titalumite`) (`KismetMathLibrary.FClamp` (* (`self.Rate`) (`self.Ore3Rate`) _returnvalue) 0.0 Ore3)))
  (set `self.Auplatite` (+ (`self.Auplatite`) (`KismetMathLibrary.FClamp` (* (`self.Rate`) (`self.Ore4Rate`) _returnvalue) 0.0 Ore4)))
  (set `self.Filler` (+ (`self.Filler`) (`KismetMathLibrary.FClamp` (* (`self.Rate`) (`self.Resource0Rate`) _returnvalue) 0.0 Resource0)))
  (set `self.Cibron` (+ (`self.Cibron`) (`KismetMathLibrary.FClamp` (* (`self.Rate`) (`self.Resource1Rate`) _returnvalue) 0.0 Resource1)))
  (set `self.Magnum` (+ (`self.Magnum`) (`KismetMathLibrary.FClamp` (* (`self.Rate`) (`self.Resource2Rate`) _returnvalue) 0.0 Resource2)))
  (set `self.Alutanium` (+ (`self.Alutanium`) (`KismetMathLibrary.FClamp` (* (`self.Rate`) (`self.Resource3Rate`) _returnvalue) 0.0 Resource3)))
  (set `self.Platigol` (+ (`self.Platigol`) (`KismetMathLibrary.FClamp` (* (`self.Rate`) (`self.Resource4Rate`) _returnvalue) 0.0 Resource4)))
  (return))

(fn `Take`
  (returns (Ore0 :type "Float (double-precision)") (Ore1 :type "Float (double-precision)") (Ore2 :type "Float (double-precision)") (Ore3 :type "Float (double-precision)") (Ore4 :type "Float (double-precision)") (Resource0 :type "Float (double-precision)") (Resource1 :type "Float (double-precision)") (Resource2 :type "Float (double-precision)") (Resource3 :type "Float (double-precision)") (Resource4 :type "Float (double-precision)"))
  (bind _returnvalue (`GameplayStatics.GetWorldDeltaSeconds`))
  (bind _irbonite (`self.Irbonite`))
  (bind _magnesite (`self.Magnesite`))
  (bind _titalumite (`self.Titalumite`))
  (bind _auplatite (`self.Auplatite`))
  (bind _filler (`self.Filler`))
  (bind _cibron (`self.Cibron`))
  (bind _magnum (`self.Magnum`))
  (bind _alutanium (`self.Alutanium`))
  (bind _platigol (`self.Platigol`))
  (bind _regolith (`self.Regolith`))
  (bind _output_get (set `self.Regolith` (- _regolith (`KismetMathLibrary.FClamp` _regolith 0.0 (* (`self.Rate`) (`self.Ore0Rate`) _returnvalue)))))
  (bind _output_get_2 (set `self.Irbonite` (- _irbonite (`KismetMathLibrary.FClamp` _irbonite 0.0 (* (`self.Rate`) (`self.Ore1Rate`) _returnvalue)))))
  (bind _output_get_3 (set `self.Magnesite` (- _magnesite (`KismetMathLibrary.FClamp` _magnesite 0.0 (* (`self.Rate`) (`self.Ore2Rate`) _returnvalue)))))
  (bind _output_get_4 (set `self.Titalumite` (- _titalumite (`KismetMathLibrary.FClamp` _titalumite 0.0 (* (`self.Rate`) (`self.Ore3Rate`) _returnvalue)))))
  (bind _output_get_5 (set `self.Auplatite` (- _auplatite (`KismetMathLibrary.FClamp` _auplatite 0.0 (* (`self.Rate`) (`self.Ore4Rate`) _returnvalue)))))
  (bind _output_get_6 (set `self.Filler` (- _filler (`KismetMathLibrary.FClamp` _filler 0.0 (* (`self.Rate`) (`self.Resource0Rate`) _returnvalue)))))
  (bind _output_get_7 (set `self.Cibron` (- _cibron (`KismetMathLibrary.FClamp` _cibron 0.0 (* (`self.Rate`) (`self.Resource1Rate`) _returnvalue)))))
  (bind _output_get_8 (set `self.Magnum` (- _magnum (`KismetMathLibrary.FClamp` _magnum 0.0 (* (`self.Rate`) (`self.Resource2Rate`) _returnvalue)))))
  (bind _output_get_9 (set `self.Alutanium` (- _alutanium (`KismetMathLibrary.FClamp` _alutanium 0.0 (* (`self.Rate`) (`self.Resource3Rate`) _returnvalue)))))
  (bind _output_get_10 (set `self.Platigol` (- _platigol (`KismetMathLibrary.FClamp` _platigol 0.0 (* (`self.Rate`) (`self.Resource4Rate`) _returnvalue)))))
  (return _output_get _output_get_2 _output_get_3 _output_get_4 _output_get_5 _output_get_6 _output_get_7 _output_get_8 _output_get_9 _output_get_10))