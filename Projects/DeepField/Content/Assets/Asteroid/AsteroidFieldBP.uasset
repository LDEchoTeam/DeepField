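; Asteroid field generator that spawns asteroids on a flat plane in distance tiers around the world origin at BeginPlay.
; Each tier scatters asteroids using random trigonometric placement, offset by a curve-weighted share of the gap to the previous tier.
; Spawns that would collide are skipped.
; Each spawned asteroid's resource container fills by tier index plus curve-weighted variance, then the asteroid updates its size and color.
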(event `self.ReceiveBeginPlay`
  (bind _returnvalue (`KismetMathLibrary.RandomFloatInRange` -180.0 180.0))
  (bind _tiers (`self.Tiers`))
  (bind _tierscale (`self.TierScale`))
  (bind _returnvalue_2 (`CurveFloat.GetFloatValue` (`self.TierDistribution`) (`KismetMathLibrary.RandomFloatInRange` 0.0 1.0)))
  (for (_array_element _array_index) _tiers
    (for _ (range 1 (+ (`self.AsteroidsPerTier`) 1))
      (bind _returnvalue_3 (+ _array_element (* _returnvalue_2 (- _array_element (`KismetMathLibrary.SelectFloat` (`|GetArrayItem` _tiers (- _array_index 1)) (`self.MinimumDistance`) (> _array_index 0))) (`self.DistanceVariance`))))
      (bind _returnvalue_4 (`|SpawnActorFromClass` "/Game/Assets/Asteroid/AsteroidBP.AsteroidBP_C" (`KismetMathLibrary.MakeTransform` (`KismetMathLibrary.MakeVector` (* _returnvalue_3 _tierscale (`KismetMathLibrary.DegCos` _returnvalue)) (* _returnvalue_3 _tierscale (`KismetMathLibrary.DegSin` _returnvalue))) (`KismetMathLibrary.RandomRotator` true)) "DontSpawnIfColliding" "OverrideRootScale" null null))
      (`/Engine/EditorBlueprintResources/StandardMacros.IsValid` _returnvalue_4
        (:`Is Valid`
          (`/Game/Assets/Resource/ResourceContainerBP.FillUp` (`/Game/Assets/Asteroid/AsteroidBP.ResourceContainer` _returnvalue_4) (+ (* _returnvalue_2 (`self.TierVariance`)) (`KismetMathLibrary.Conv_IntToDouble` _array_index)))
          (`/Game/Assets/Asteroid/AsteroidBP.Resize` _returnvalue_4)
          (`/Game/Assets/Asteroid/AsteroidBP.Recolor` _returnvalue_4))))))

(fn `UserConstructionScript`)