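; Asteroid actor whose mesh scale and color reflect the size and color of its ResourceContainer.
; Resize and Recolor run on BeginPlay and are separate events, with color driven through a dynamic material instance.
; Latched disables sphere collision and optionally records the gap beyond the asteroid's radius; Unlatched restores both.
; Shift places the asteroid at radius plus that gap from a reference point, using a supplied normal if direction degenerates.
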(event `self.ReceiveBeginPlay`
  (set `self.CollisionProfileName` (`PrimitiveComponent.GetCollisionProfileName` (`self.SphereCol`)))
  (bind _returnvalue (`PrimitiveComponent.CreateDynamicMaterialInstance` (`self.StaticMesh`) 0 null "None"))
  (set `self.MaterialInstance` _returnvalue)
  (`self.Resize`)
  (`self.Recolor`))

(event `Latched`
  (params (Reference :type "Vector Structure") (NoExtraRadius :type Boolean))
  (bind _size (`/Game/Assets/Resource/ResourceContainerBP.GetSize` (`self.ResourceContainer`)))
  (set `self.ExtraRadius` (`KismetMathLibrary.SelectFloat` 0.0 (- (`KismetMathLibrary.VSize` (- (`self.K2_GetActorLocation`) Reference)) (* (+ _size (`self.BaseSize`)) (`self.Radius`))) NoExtraRadius))
  (`PrimitiveComponent.SetCollisionProfileName` (`self.SphereCol`) "NoCollision" true))

(event `Unlatched`
  (set `self.ExtraRadius` 0.0)
  (`PrimitiveComponent.SetCollisionProfileName` (`self.SphereCol`) (`self.CollisionProfileName`) true))

(event `Resize`
  (bind _size (`/Game/Assets/Resource/ResourceContainerBP.GetSize` (`self.ResourceContainer`)))
  (bind _returnvalue (+ _size (`self.BaseSize`)))
  (`SceneComponent.SetWorldScale3D` (`self.StaticMesh`) (`KismetMathLibrary.MakeVector` _returnvalue _returnvalue _returnvalue)))

(event `Shift`
  (params (Reference :type "Vector Structure") (Normal :type "Vector Structure"))
  (bind _returnvalue (`KismetMathLibrary.Normal` (- (`self.K2_GetActorLocation`) Reference)))
  (`self.K2_SetActorLocation` (+ Reference (* (`KismetMathLibrary.SelectVector` _returnvalue Normal (> (`KismetMathLibrary.VSize` _returnvalue) 0.0001)) (+ (* (+ (stale `Resize` _size) (`self.BaseSize`)) (`self.Radius`)) (`self.ExtraRadius`))))))

(event `Recolor`
  (bind _color (`/Game/Assets/Resource/ResourceContainerBP.GetColor` (`self.ResourceContainer`)))
  (`MaterialInstanceDynamic.SetVectorParameterValue` (`self.MaterialInstance`) "ResourceColor" (`KismetMathLibrary.Conv_ColorToLinearColor` _color)))

(fn `UserConstructionScript`)