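; BaseBP is a Blueprint actor for a base that can be latched and unlatched and carries a BoxCollision and a sized ResourceContainer.
; Latching disables box collision and sets ExtraRadius to zero or to the distance from a reference point minus the size-scaled Radius.
; Unlatching zeroes ExtraRadius and restores the collision profile cached at BeginPlay.
; A Create event adds a static mesh component using the Base mesh.
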(event `self.ReceiveBeginPlay`
  (set `self.CollisionProfileName` (`PrimitiveComponent.GetCollisionProfileName` (`self.BoxCollision`))))

(event `Latched`
  (params (Reference :type "Vector Structure") (NoExtraRadius :type Boolean))
  (bind _size (`/Game/Assets/Resource/ResourceContainerBP.GetSize` (`self.ResourceContainer`)))
  (set `self.ExtraRadius` (`KismetMathLibrary.SelectFloat` 0.0 (- (`KismetMathLibrary.VSize` (- (`self.K2_GetActorLocation`) Reference)) (* (+ _size (`self.BaseSize`)) (`self.Radius`))) NoExtraRadius))
  (`PrimitiveComponent.SetCollisionProfileName` (`self.BoxCollision`) "NoCollision" true))

(event `Unlatched`
  (set `self.ExtraRadius` 0.0)
  (`PrimitiveComponent.SetCollisionProfileName` (`self.BoxCollision`) (`self.CollisionProfileName`) true))

(event `Create`
  (bind _returnvalue (`|AddComponentByClass` "/Script/Engine.StaticMeshComponent"))
  (`StaticMeshComponent.SetStaticMesh` _returnvalue "/Game/Assets/Base/Base.Base"))

(fn `UserConstructionScript`)