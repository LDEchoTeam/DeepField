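; Player-controlled miner ship that latches onto asteroids to strip them or build them back up, with its own camera and overlay.
; Tick drives swept movement and rate-limited turning with thruster effects, both slowed by the grabbed asteroid's size.
; Latch attaches or releases an overlapping asteroid.
; While held, Mine and Build move resources between the ship and asteroid containers, resizing, shifting and recoloring the asteroid, or destroying or spawning it as needed.
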(event `self.ReceiveBeginPlay`
  (bind _camera (`self.Camera`))
  (bind _asplayer_controller (cast `PlayerController` (`self.GetController`)))
  (`PlayerController.SetViewTargetWithBlend` _asplayer_controller _camera 0.0 "VTBlend_Linear" 0.0 false)
  (set `/Game/Assets/Miner/CameraBP.Bitch` self _camera)
  (`/Game/Assets/Resource/ResourceContainerBP.Format` (`self.ResourceContainer`))
  (bind _returnvalue (`|CreateWidget` "/Game/Assets/Interface/Overlay.Overlay_C"))
  (bind _output_get (set `self.Overlay` _returnvalue))
  (`UserWidget.AddToViewport` _output_get 0))

(event `self.ReceiveTick`
  (params (DeltaSeconds :type "Float (single-precision)"))
  (`self.Move`)
  (`self.Mine`)
  (`self.Build`))

(event `Move`
  (bind _blast1 (`self.Blast1`))
  (bind _blast2 (`self.Blast2`))
  (bind _returnvalue (`KismetMathLibrary.MakeVector2D` (`self.GetInputAxisValue`) (`self.GetInputAxisValue`)))
  (bind _yaw (.yaw (`self.K2_GetActorRotation`)))
  (bind _returnvalue_2 (`KismetMathLibrary.VSize2D` _returnvalue))
  (bind _returnvalue_3 (- (.yaw (`KismetMathLibrary.Conv_VectorToRotator` (`KismetMathLibrary.Conv_Vector2DToVector` _returnvalue))) _yaw))
  (bind _returnvalue_4 (`KismetMathLibrary.SelectFloat` (- _returnvalue_3 360.0) _returnvalue_3 (> _returnvalue_3 359.0)))
  (if (> _returnvalue_2 0.1)
    (`|ExecutionSequence`
      (:`then_0`
        (`ActorComponent.Activate` _blast1 false)
        (`ActorComponent.Activate` _blast2 false))
      (:`then_1`
        (if (`self.Grabbing`)
          (bind _size (`/Game/Assets/Resource/ResourceContainerBP.GetSize` (`/Game/Assets/Asteroid/AsteroidBP.ResourceContainer` (`self.LastGrabbedBitch`)))))
        (bind _returnvalue_5 (`KismetMathLibrary.SafeDivide` (`self.Power`) (+ (`KismetMathLibrary.SelectFloat` _size 0.0 (`self.Grabbing`)) (`self.Size`))))
        (bind _sweephitresult (`self.K2_SetActorLocation` (+ (`self.K2_GetActorLocation`) (`KismetMathLibrary.Conv_Vector2DToVector` (* (`KismetMathLibrary.Normal2D` _returnvalue) (* (`KismetMathLibrary.FClamp` _returnvalue_2) _returnvalue_5)))) true))
        (if (not (`GameplayStatics.BreakHitResult` _sweephitresult))
          (`|ExecutionSequence`
            (:`then_0`
              _)
            (:`then_1`
              (bind _returnvalue_6 (* _returnvalue_5 (`self.RotationPowerFraction`)))
              (`self.K2_SetActorRotation` (`KismetMathLibrary.MakeRotator` (.roll (`self.K2_GetActorRotation`)) (.pitch (`self.K2_GetActorRotation`)) (+ _yaw (`KismetMathLibrary.FClamp` (+ (- _returnvalue_3 (* (`KismetMathLibrary.Conv_BoolToDouble` (> _returnvalue_3 180.0)) 360.0)) (* (`KismetMathLibrary.Conv_BoolToDouble` (< _returnvalue_3 -180.0)) 360.0)) (* _returnvalue_6 -1.0) _returnvalue_6))))))
          (if (< _returnvalue_4 -0.0001)
            (`ActorComponent.Activate` (`self.Puff1`) false)
            (`ActorComponent.Activate` (`self.Puff3`) false)
            (elif (> _returnvalue_4 0.0001)
              (`ActorComponent.Activate` (`self.Puff2`) false)
              (`ActorComponent.Activate` (`self.Puff4`) false))))))
    (else
      (`ActorComponent.Deactivate` _blast1)
      (`ActorComponent.Deactivate` _blast2))))

(event `InputAction|Latch`
  (params (Key :type "Key Structure"))
  (bind _lastgrabbedbitch (`self.LastGrabbedBitch`))
  (bind _overlappingactors (`PrimitiveComponent.GetOverlappingActors` (`self.LatchRange`) "/Game/Assets/Asteroid/AsteroidBP.AsteroidBP_C"))
  (:`Pressed`
    (if (`self.Grabbing`)
      (`self.K2_DetachFromActor` (`self.LastGrabbedBitch`) "KeepWorld" "KeepWorld" "KeepWorld")
      (set `self.Grabbing` false)
      (`/Game/Assets/Asteroid/AsteroidBP.Unlatched` _lastgrabbedbitch)
      (elif (> (`KismetArrayLibrary.Array_Length` _overlappingactors) 0)
        (bind _asasteroid_bp (cast `/Game/Assets/Asteroid/AsteroidBP` (`|GetArrayItem` _overlappingactors)))
        (bind _output_get (set `self.LastGrabbedBitch` _asasteroid_bp))
        (`self.K2_AttachToActor` _output_get self "None" "KeepWorld" "KeepWorld" "KeepWorld" true)
        (set `self.Grabbing` true)
        (`/Game/Assets/Asteroid/AsteroidBP.Latched` _lastgrabbedbitch (`SceneComponent.K2_GetComponentLocation` (`self.LatchPoint`)) false)))))

(event `InputAction|Mine`
  (params (Key :type "Key Structure"))
  (bind _suck (`self.Suck`))
  (:`Pressed`
    (set `self.Mining` true)
    (if (`self.Grabbing`)
      (`ActorComponent.Activate` _suck false)))
  (:`Released`
    (set `self.Mining` false)
    (`ActorComponent.Deactivate` _suck)))

(event `Mine`
  (bind _resourcecontainer (`self.ResourceContainer`))
  (bind _lastgrabbedbitch (`self.LastGrabbedBitch`))
  (bind _resourcecontainer_2 (`/Game/Assets/Asteroid/AsteroidBP.ResourceContainer` _lastgrabbedbitch))
  (if (and (`self.Grabbing`) (`self.Mining`))
    (bind (_ore0 _ore1 _ore2 _ore3 _ore4 _resource0 _resource1 _resource2 _resource3 _resource4) (`/Game/Assets/Resource/ResourceContainerBP.Take` _resourcecontainer_2))
    (bind _yes (`/Game/Assets/Resource/ResourceContainerBP.IsEmpty` _resourcecontainer_2))
    (if _yes
      (`self.K2_DestroyActor` _lastgrabbedbitch)
      (set `self.Grabbing` false)
      (`ActorComponent.Deactivate` (`self.Suck`))
      (else
        (`/Game/Assets/Asteroid/AsteroidBP.Resize` _lastgrabbedbitch)
        (`/Game/Assets/Asteroid/AsteroidBP.Shift` _lastgrabbedbitch (`SceneComponent.K2_GetComponentLocation` (`self.LatchPoint`)) (`self.GetActorForwardVector`))
        (`/Game/Assets/Asteroid/AsteroidBP.Recolor` _lastgrabbedbitch)))
    (`/Game/Assets/Resource/ResourceContainerBP.Put` _resourcecontainer _ore0 _ore1 _ore2 _ore3 _ore4 _resource0 _resource1 _resource2 _resource3 _resource4)
    (`/Game/Assets/Resource/ResourceContainerBP.Format` _resourcecontainer)))

(event `InputAction|Build`
  (params (Key :type "Key Structure"))
  (:`Pressed`
    (set `self.Building` true))
  (:`Released`
    (set `self.Building` false)
    (`ActorComponent.Deactivate` (`self.Blow`) :!label _label)))

(event `Build`
  (bind _lastgrabbedbitch (`self.LastGrabbedBitch`))
  (if (`self.Building`)
    (bind _yes (`/Game/Assets/Resource/ResourceContainerBP.IsEmpty` (`self.ResourceContainer`)))
    (if _yes
      (goto _label)
      (else
        (`ActorComponent.Activate` (`self.Blow`) false)
        (if (not (`self.Grabbing`))
          (bind _returnvalue (`|SpawnActorFromClass` "/Game/Assets/Asteroid/AsteroidBP.AsteroidBP_C" (`KismetMathLibrary.MakeTransform` (.location (`SceneComponent.K2_GetComponentToWorld` (`self.LatchPoint`))) (`KismetMathLibrary.RandomRotator` true) (.scale (`SceneComponent.K2_GetComponentToWorld` (`self.LatchPoint`)))) "AlwaysSpawn" "OverrideRootScale" null null))
          (bind _output_get (set `self.LastGrabbedBitch` _returnvalue))
          (`self.K2_AttachToActor` _output_get self "None" "KeepWorld" "KeepWorld" "KeepWorld" true)
          (`/Game/Assets/Asteroid/AsteroidBP.Latched` _output_get (`SceneComponent.K2_GetComponentLocation` (`self.LatchPoint`)) true)
          (set `self.Grabbing` true))
        (bind (_ore0 _ore1 _ore2 _ore3 _ore4 _resource0 _resource1 _resource2 _resource3 _resource4) (`/Game/Assets/Resource/ResourceContainerBP.Take` (`self.ResourceContainer`)))
        (`/Game/Assets/Resource/ResourceContainerBP.Put` (`/Game/Assets/Asteroid/AsteroidBP.ResourceContainer` _lastgrabbedbitch) _ore0 _ore1 _ore2 _ore3 _ore4 _resource0 _resource1 _resource2 _resource3 _resource4)
        (`/Game/Assets/Asteroid/AsteroidBP.Resize` _lastgrabbedbitch)
        (`/Game/Assets/Asteroid/AsteroidBP.Shift` _lastgrabbedbitch (`SceneComponent.K2_GetComponentLocation` (`self.LatchPoint`)) (`self.GetActorForwardVector`))
        (`/Game/Assets/Asteroid/AsteroidBP.Recolor` _lastgrabbedbitch)
        (`/Game/Assets/Resource/ResourceContainerBP.Format` (`self.ResourceContainer`))))))

(fn `UserConstructionScript`)